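; BP_DamageFlash is an actor component that briefly flashes its owner's skeletal mesh when the owner takes damage.
; On BeginPlay it binds to OnTakeAnyDamage, creates a dynamic material instance on the mesh's first material slot and caches the original emissive color and multiplier.
; The DamageFlash event applies the flash color and intensity, waits for the flash duration with a Delay, then restores the cached values.
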(event Custom|DamageFlash
  (params (DamagedActor :type Actor%20Object%20Reference) (Damage :type Float%20%28single-precision%29) (DamageType :type Damage%20Type%20Object%20Reference) (InstigatedBy :type Controller%20Object%20Reference) (DamageCauser :type Actor%20Object%20Reference))
  (bind _flashmat (Variables|Initialization|GetFlashMat))
  (bind _flashmat_2 (Variables|Initialization|GetFlashMat))
  ;[1 1 1] Set Flash Values
  (Rendering|Material|SetVectorParameterValue _flashmat_2 "EmissiveColor" (Variables|FlashSettings|GetFlashColor) :!class /Script/Engine.MaterialInstanceDynamic)
  (Rendering|Material|SetScalarParameterValue _flashmat_2 "EmissiveMultiplier" (Variables|FlashSettings|GetFlashIntensity) :!class /Script/Engine.MaterialInstanceDynamic)
  (Utilities|FlowControl|Delay (Variables|FlashSettings|GetFlashDuration))
  ;[1 1 1] Return to Original Values
  (Rendering|Material|SetVectorParameterValue _flashmat "EmissiveColor" (Variables|Initialization|GetInitEmissiveColor) :!class /Script/Engine.MaterialInstanceDynamic)
  (Rendering|Material|SetScalarParameterValue _flashmat "EmissiveMultiplier" (Variables|Initialization|GetInitEmissiveMultiplier) :!class /Script/Engine.MaterialInstanceDynamic))

(event EventBeginPlay
  (bind _returnvalue (Components|GetOwner))
  (Variables|Initialization|SetOwner _returnvalue)
  (EventDispatchers|BindEventtoOnTakeAnyDamage _returnvalue (EventDispatchers|CreateEvent :!event Custom|DamageFlash))
  ;[1 1 1] Setup Dynamic Material Instance from Actor
  (Utilities|IsValid (Actor|GetComponentbyClass (Variables|Initialization|GetOwner) "/Script/Engine.SkeletalMeshComponent")
    (:Is%20Valid
      (bind _returnvalue_2 (Rendering|Material|CreateDynamicMaterialInstance (Actor|GetComponentbyClass (Variables|Initialization|GetOwner) "/Script/Engine.SkeletalMeshComponent") 0 0 "None" :!class /Script/Engine.PrimitiveComponent))
      (Variables|Initialization|SetFlashMat _returnvalue_2)
      ;[1 1 1] Get Initial Emissive Values
      (bind _returnvalue_3 (Rendering|Material|GetVectorParameterValue (Variables|Initialization|GetFlashMat) "EmissiveColor" :!class /Script/Engine.MaterialInstanceDynamic))
      (Variables|Initialization|SetInitEmissiveColor _returnvalue_3)
      (bind _returnvalue_4 (Rendering|Material|GetScalarParameterValue (Variables|Initialization|GetFlashMat) "EmissiveMultiplier" :!class /Script/Engine.MaterialInstanceDynamic))
      (Variables|Initialization|SetInitEmissiveMultiplier _returnvalue_4))))