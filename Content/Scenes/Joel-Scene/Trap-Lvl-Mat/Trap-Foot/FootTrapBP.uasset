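; Foot trap that immobilizes the top-down player character on overlap, plays a sound and spawns a temporary TrapRed actor beneath them.
; Once triggered, it follows the player's mesh on Tick, then releases them after a short delay by restoring walking.
; It then either destroys itself or re-arms its collision later, with a timeline driving open and close.
; While untriggered in NormalMove, InterpToMovement moves it toward a randomized nearby point set at construction.
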(event OnComponentBeginOverlap(Cylinder)
  (params (OverlappedComponent :type Primitive%20Component%20Object%20Reference) (OtherActor :type Actor%20Object%20Reference) (OtherComp :type Primitive%20Component%20Object%20Reference) (OtherBodyIndex :type Integer) (bFromSweep :type Boolean) (SweepResult :type Hit%20Result%20Structure%20%28by%20ref%29))
  (bind _asbp_top_down_character (Utilities|Casting|CastToBP_TopDownCharacter OtherActor))
  (Utilities|FlowControl|Delay 0.2)
  (CallFunction|CatchPlayer _asbp_top_down_character)
  (Input|EnableInput (Game|GetPlayerController 0))
  (Collision|SetCollisionEnabled (Variables|Default|GetCylinder) "NoCollision")
  (CallFunction|GotoPlayer)
  (Audio|PlaySound2D "/Game/Sounds/PlantRed_Cue.PlantRed_Cue" 1.0 1.0 0.0 0 0)
  (bind _returnvalue (Game|SpawnActorfromClass "/Game/Scenes/Joel-Scene/Trap-Lvl-Mat/Trap-Foot/TrapRed.TrapRed_C" (Math|Conversions|ToTransform(Vector) (- (.Location (Math|Transform|BreakTransform (Transformation|GetWorldTransform (Variables|/Script/Engine.Actor|GetRootComponent _asbp_top_down_character)))) (Math|Vector|MakeVector 0.0 0.0 1e+02))) "Undefined" 0 0))
  (Utilities|FlowControl|Delay 2.0)
  (CallFunction|Open)
  (Actor|DestroyActor _returnvalue)
  (if (Variables|Default|GetDestroyAfterUse)
    (Actor|DestroyActor))
  (if (Utilities|IsValid (Components|GetOwner))
    (Timeline|Open/Close%20Foot%20Trap Play)))

(event Custom|Catch%20Player
  (params (Character :type Character%20Object%20Reference))
  (Pawn|Components|CharacterMovement|DisableMovement (Variables|/Script/Engine.Character|GetCharacterMovement Character)))

(event Custom|Open
  (Pawn|Components|CharacterMovement|SetMovementMode (Variables|/Script/Engine.Character|GetCharacterMovement (stale OnComponentBeginOverlap(Cylinder) _asbp_top_down_character)) "MOVE_Walking" 0)
  (Utilities|FlowControl|Sequence
    (:then_0
      (Timeline|Open/Close%20Foot%20Trap Reverse))
    (:then_1
      (Utilities|FlowControl|Delay 3.0)
      (Collision|SetCollisionEnabled (Variables|Default|GetCylinder) "QueryAndPhysics"))))

(event Custom|GoToPlayer
  (Variables|Default|SetNormalMove false))

(event EventTick
  (params (DeltaSeconds :type Float%20%28single-precision%29))
  (if (not (Variables|Default|GetNormalMove))
    (Transformation|SetActorLocation (Transformation|GetWorldLocation (Variables|/Script/Engine.Character|GetMesh (stale OnComponentBeginOverlap(Cylinder) _asbp_top_down_character))) false false)))

(fn ConstructionScript
  (if (Variables|Default|GetNormalMove)
    (Class|InterptoMovementComponent|AddControlPointPosition (Variables|Default|GetInterpToMovement) "0, 0, 0" true)
    (Class|InterptoMovementComponent|AddControlPointPosition (Variables|Default|GetInterpToMovement) (Math|Vector|MakeVector (Math|Random|RandomFloatinRange -1e+02 1e+02) (Math|Random|RandomFloatinRange -1e+02 1e+02) (Math|Random|RandomFloatinRange 0.0 1e+01)) true)))