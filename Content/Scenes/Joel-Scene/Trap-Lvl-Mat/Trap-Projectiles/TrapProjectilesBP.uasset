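; Trap actor that fires a short volley of projectiles when another actor overlaps it.
; On overlap it plays a press sound, then spawns three Projectile2 actors in staggered succession from three spawn-point components, using their world location and rotation.
; A CanSpawn flag blocks retriggering during the volley and re-arms after a cooldown of a few seconds.
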(event EventBeginPlay)

(event Collision|EventActorBeginOverlap
  (params (OtherActor :type Actor%20Object%20Reference))
  (bind _spawnbuller (Variables|Default|GetSpawnBuller))
  (bind _spawn_bullet (Variables|Default|GetSpawn%20Bullet))
  (bind _spawn_bullet1 (Variables|Default|GetSpawn%20Bullet1))
  (if (Variables|Default|Getcan%20spawn?)
    (Variables|Default|Setcan%20spawn? false)
    (Audio|PlaySound2D "/Game/Sounds/Trap_O_Press_Cue.Trap_O_Press_Cue" 1.0 1.0 0.0 0 0)
    (Utilities|FlowControl|Delay 0.2)
    (Game|SpawnActorfromClass "/Game/TopDown/Blueprints/Projectile2.Projectile2_C" (Math|Transform|MakeTransform (Transformation|GetWorldLocation _spawnbuller) (Transformation|GetWorldRotation _spawnbuller)) "Undefined" 0 0)
    (Utilities|FlowControl|Delay 0.1)
    (Game|SpawnActorfromClass "/Game/TopDown/Blueprints/Projectile2.Projectile2_C" (Math|Transform|MakeTransform (Transformation|GetWorldLocation _spawn_bullet) (Transformation|GetWorldRotation _spawn_bullet)) "Undefined" 0 0)
    (Utilities|FlowControl|Delay 0.05)
    (Game|SpawnActorfromClass "/Game/TopDown/Blueprints/Projectile2.Projectile2_C" (Math|Transform|MakeTransform (Transformation|GetWorldLocation _spawn_bullet1) (Transformation|GetWorldRotation _spawn_bullet1)) "Undefined" 0 0)
    (Utilities|FlowControl|Delay 0.2)
    (Utilities|FlowControl|Delay 3.0)
    (Variables|Default|Setcan%20spawn? true)))

(event EventTick
  (params (DeltaSeconds :type Float%20%28single-precision%29)))

(fn ConstructionScript)